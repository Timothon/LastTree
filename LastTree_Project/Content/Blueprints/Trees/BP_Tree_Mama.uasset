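; BP_Tree_Mama is a tree Blueprint for the "Mama" tree that registers itself with the player character.
; On BeginPlay it runs the parent logic, casts player character 0 to BP_ThirdPersonCharacter and stores itself in that character's MamaTreeRef.
; The construction script only calls the parent, and the overlap and tick events are disabled.
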(event EventBeginPlay
  (|CallParentFunction)
  (bind _asbp_third_person_character (Utilities|Casting|CastToBP_ThirdPersonCharacter (Game|GetPlayerCharacter 0)))
  (Variables|/Game/ThirdPerson/Blueprints/BP_ThirdPersonCharacter.BP_ThirdPersonCharacter_C|SetMamaTreeRef _asbp_third_person_character self))

(event Collision|EventActorBeginOverlap
  (params (OtherActor :type Actor%20Object%20Reference))
  (|CallParentFunction OtherActor) ; This node is disabled and will not be called.\nDrag off pins to build functionality.
)

(event EventTick
  (params (DeltaSeconds :type Float%20%28single-precision%29))
  (|CallParentFunction DeltaSeconds) ; This node is disabled and will not be called.\nDrag off pins to build functionality.
)

(fn ConstructionScript
  (|CallParentFunction))