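; Base tree actor that shifts between neutral, decaying and rejuvenated states, swapping material to match.
; Enemy contact kills the enemy and costs health; at zero the tree decays, launching nearby enemies and removing any player range it granted.
; A player dash rejuvenates it, restoring health, killing overlapping enemies and extending MaxDistanceFromMama.
; While decaying, large and massive trees spawn enemies around themselves through a Tick-driven Delay, faster during fury spawning.
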(event OnComponentBeginOverlap(Capsule)
  (params (OverlappedComponent :type Primitive%20Component%20Object%20Reference) (OtherActor :type Actor%20Object%20Reference) (OtherComp :type Primitive%20Component%20Object%20Reference) (OtherBodyIndex :type Integer) (bFromSweep :type Boolean) (SweepResult :type Hit%20Result%20Structure%20%28by%20ref%29))
  (bind _asbp_enemy (Utilities|Casting|CastToBP_Enemy OtherActor)
    (:then
      (if (== (Variables|/Script/Engine.Character|GetCapsuleComponent _asbp_enemy) OtherComp)
        (if (and (not (Utilities|Enum|Equal(Enum) (Variables|Default|GetStateOfDecay) "NewEnumerator2")) (not (Utilities|Enum|Equal(Enum) (Variables|Default|GetTreeType/Size) "NewEnumerator3")))
          (Default|EnemyKilled _asbp_enemy)
          (bind _output_get (Variables|Default|SetHealthRemaining (- (Variables|Default|GetHealthRemaining) 1)))
          (if (<= _output_get 0)
            (Utilities|FlowControl|Sequence
              (:then_0
                (if (Utilities|Enum|Equal(Enum) (Variables|Default|GetStateOfDecay) "NewEnumerator0")
                  (bind _asbp_third_person_character (Utilities|Casting|CastToBP_ThirdPersonCharacter (Game|GetPlayerCharacter 0)))
                  (Variables|/Game/ThirdPerson/Blueprints/BP_ThirdPersonCharacter.BP_ThirdPersonCharacter_C|SetMaxDistanceFromMama _asbp_third_person_character (- (Variables|/Game/ThirdPerson/Blueprints/BP_ThirdPersonCharacter.BP_ThirdPersonCharacter_C|GetMaxDistanceFromMama _asbp_third_person_character) (Variables|Default|GetRangeGive/Taken)))))
              (:then_1
                (Variables|Default|SetStateOfDecay "NewEnumerator2")
                (CallFunction|OnDecayed)
                (for _array_element (Collision|GetOverlappingActors (Variables|Default|GetCapsule) "/Game/Blueprints/BP_Enemy.BP_Enemy_C" :!class /Script/Engine.PrimitiveComponent)
                  (bind _asbp_enemy_2 (Utilities|Casting|CastToBP_Enemy _array_element))
                  (Character|LaunchCharacter _asbp_enemy_2 (Math|Vector|MakeVector (.x (* (Math|Vector|Normalize (- (Transformation|GetActorLocation _array_element) (Transformation|GetActorLocation))) (Math|Float|MakeLiteralFloat 4e+02))) (.y (* (Math|Vector|Normalize (- (Transformation|GetActorLocation _array_element) (Transformation|GetActorLocation))) (Math|Float|MakeLiteralFloat 4e+02))) 2e+02) false false))))))))
    (:CastFailed
      (bind _asbp_third_person_character_2 (Utilities|Casting|CastToBP_ThirdPersonCharacter OtherActor))
      (if (and (Variables|/Game/ThirdPerson/Blueprints/BP_ThirdPersonCharacter.BP_ThirdPersonCharacter_C|GetIsDashing _asbp_third_person_character_2) (== (Variables|/Script/Engine.Character|GetCapsuleComponent _asbp_third_person_character_2) OtherComp))
        (if (and (not (Utilities|Enum|Equal(Enum) (Variables|Default|GetStateOfDecay) "NewEnumerator0")) (not (Utilities|Enum|Equal(Enum) (Variables|Default|GetTreeType/Size) "NewEnumerator2")))
          (Variables|Default|SetHealthRemaining (.HealthRemaining (Utilities|GetClassDefaults (Utilities|GetClass self))))
          (Variables|Default|SetStateOfDecay "NewEnumerator0")
          (Variables|/Script/Engine.MovementComponent|SetVelocity (Variables|/Script/Engine.Character|GetCharacterMovement _asbp_third_person_character_2) "0, 0, 0")
          (Utilities|FlowControl|Sequence
            (:then_0
              (CallFunction|OnRejuvinated)
              (for _array_element_2 (Collision|GetOverlappingActors (Variables|Default|GetCapsule) "/Game/Blueprints/BP_Enemy.BP_Enemy_C" :!class /Script/Engine.PrimitiveComponent)
                (bind _asbp_enemy_3 (Utilities|Casting|CastToBP_Enemy _array_element_2))
                (Default|EnemyKilled _asbp_enemy_3)))
            (:then_1
              (bind _asbp_third_person_character_3 (Utilities|Casting|CastToBP_ThirdPersonCharacter (Game|GetPlayerCharacter 0)))
              (Variables|/Game/ThirdPerson/Blueprints/BP_ThirdPersonCharacter.BP_ThirdPersonCharacter_C|SetMaxDistanceFromMama _asbp_third_person_character_3 (+ (Variables|/Game/ThirdPerson/Blueprints/BP_ThirdPersonCharacter.BP_ThirdPersonCharacter_C|GetMaxDistanceFromMama _asbp_third_person_character_3) (Variables|Default|GetRangeGive/Taken))))))))))

(event Custom|OnDecayed
  (CallFunction|SetMaterialbyState))

(event Custom|OnRejuvinated
  (CallFunction|SetMaterialbyState))

(event EventBeginPlay
  (CallFunction|SetMaterialbyState))

(event Collision|EventActorBeginOverlap
  (params (OtherActor :type Actor%20Object%20Reference)))

(event EventTick
  (params (DeltaSeconds :type Float%20%28single-precision%29))
  (bind _spawnrate (Variables|Default|GetSpawnRate))
  (if (Utilities|Enum|Equal(Enum) (Variables|Default|GetStateOfDecay) "NewEnumerator2")
    (Utilities|FlowControl|Delay (select (Variables|Default|GetIsFurySpawning) (/ _spawnrate 2.0) _spawnrate))
    (switch Utilities|FlowControl|Switch|SwitchonE_TreeType (Variables|Default|GetTreeType/Size)
      (:NewEnumerator1
        _)
      (:NewEnumerator3
        _))
    (CallFunction|SpawnEnemy)))

(fn ConstructionScript)

(fn SetMaterialbyState
  (bind _treestaticmesh (Variables|Default|GetTreeStaticMesh))
  (switch Utilities|FlowControl|Switch|SwitchonE_TreeState (Variables|Default|GetStateOfDecay)
    (:NewEnumerator0
      (Rendering|Material|SetMaterial _treestaticmesh 0 "/Engine/VREditor/UI/ArrowMaterial.ArrowMaterial"))
    (:NewEnumerator1
      (Rendering|Material|SetMaterial _treestaticmesh 0 "/Engine/MapTemplates/Materials/BasicAsset03.BasicAsset03"))
    (:NewEnumerator2
      (Rendering|Material|SetMaterial _treestaticmesh 0 "/Engine/MapTemplates/Materials/BasicAsset01.BasicAsset01"))))

(fn SpawnEnemy
  (bind _returnvalue (Math|Random|RandomRotator false))
  (bind _self self)
  (bind _capsule (Variables|Default|GetCapsule))
  (bind _returnvalue_2 (Math|Vector|GetForwardVector _returnvalue))
  (bind _returnvalue_3 (Transformation|GetActorLocation _self))
  (bind _capsuleradius (Variables|/Script/Engine.CapsuleComponent|GetCapsuleRadius _capsule))
  (bind _returnvalue_4 (+ _capsuleradius 2e+02))
  (bind _returnvalue_5 (* _returnvalue_2 _returnvalue_4))
  (bind _returnvalue_6 (+ _returnvalue_3 _returnvalue_5))
  (Game|SpawnActorfromClass "/Game/Blueprints/BP_Enemy.BP_Enemy_C" (Math|Transform|MakeTransform (Math|Vector|MakeVector (.x _returnvalue_6) (.y _returnvalue_6) (.z (Transformation|GetActorLocation self))) "0, 0, 0" "1.000000,1.000000,1.000000") "Undefined" 0 0))