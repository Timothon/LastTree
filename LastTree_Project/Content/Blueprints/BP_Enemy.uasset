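; Enemy that picks a target tree on spawn and destroys itself when killed.
; GetClosestTree takes the nearest overlapping tree not in an excluded decay state, falling back to the player's Mama tree reference.
; Tick and a looping timer both billboard the Cylinder toward the player's follow camera.
; The AIMoveTo and manual offset movement toward that tree are disconnected, so this graph never moves the enemy.
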(event Custom|EnemyKilled
  (Actor|DestroyActor))

(event Custom|Enemy%20Visibility%20Check
  (bind _asbp_third_person_character (Utilities|Casting|CastToBP_ThirdPersonCharacter (Game|GetPlayerCharacter 0)))
  (Transformation|SetWorldRotation (Variables|Default|GetCylinder) (Math|Rotator|FindLookatRotation (Transformation|GetActorLocation) (Transformation|GetWorldLocation (Variables|/Game/ThirdPerson/Blueprints/BP_ThirdPersonCharacter.BP_ThirdPersonCharacter_C|GetFollowCamera _asbp_third_person_character))) false false))

(event EventBeginPlay
  (CallFunction|GetClosestTree)
  (Utilities|Time|SetTimerbyEvent (delegate Custom|Enemy%20Visibility%20Check) 0.05 true))

(event Collision|EventActorBeginOverlap
  (params (OtherActor :type Actor%20Object%20Reference)))

(event EventTick
  (params (DeltaSeconds :type Float%20%28single-precision%29))
  (bind _asbp_third_person_character (Utilities|Casting|CastToBP_ThirdPersonCharacter (Game|Player|GetPlayerPawn 0)))
  (Transformation|SetWorldRotation (Variables|Default|GetCylinder) (Math|Rotator|FindLookatRotation (Transformation|GetActorLocation) (Transformation|GetWorldLocation (Variables|/Game/ThirdPerson/Blueprints/BP_ThirdPersonCharacter.BP_ThirdPersonCharacter_C|GetFollowCamera _asbp_third_person_character))) false false))

(fn ConstructionScript)

(fn GetClosestTree
  (for _array_element (Collision|GetOverlappingActors (Variables|Default|GetSphere) "/Game/Blueprints/Trees/BP_Tree_Base.BP_Tree_Base_C" :!class /Script/Engine.PrimitiveComponent)
    (bind _asbp_tree_base (Utilities|Casting|CastToBP_Tree_Base _array_element))
    (if (Utilities|Enum|NotEqual(Enum) (Variables|/Game/Blueprints/Trees/BP_Tree_Base.BP_Tree_Base_C|GetStateOfDecay _asbp_tree_base) "NewEnumerator2")
      (if (< (Math|Vector|Distance(Vector) (Transformation|GetActorLocation _asbp_tree_base) (Transformation|GetWorldLocation (Variables|Collision|GetCapsuleComponent))) (LocalVariables|GetClosestDistance))
        (LocalVariables|SetClosestDistance (Math|Vector|Distance(Vector) (Transformation|GetActorLocation _asbp_tree_base) (Transformation|GetWorldLocation (Variables|Collision|GetCapsuleComponent))))
        (Variables|Default|SetClosestTree _asbp_tree_base))))
  (if (== (LocalVariables|GetClosestDistance) 9e+03)
    (bind _asbp_third_person_character (Utilities|Casting|CastToBP_ThirdPersonCharacter (Game|GetPlayerCharacter 0)))
    (Variables|Default|SetClosestTree (Variables|/Game/ThirdPerson/Blueprints/BP_ThirdPersonCharacter.BP_ThirdPersonCharacter_C|GetMamaTreeRef _asbp_third_person_character))))